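; Game mode for a VR shooting range that runs a timed round and keeps a saved high score.
; BeginPlay finds the moving target, timer and high score actors by interface, then shows the score loaded from the SaveScore slot.
; StartGame enables scoring and target movement, counting down one minute through a Delay loop.
; At zero it stops both and saves the pawn's score if it beats the loaded maximum.
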(event EventBeginPlay
  ;[1 1 1] Move movable targets
  (bind _outactors (Actor|GetAllActorswithInterface "/Game/Blueprints/Interface/BPI_MovableTarget.BPI_MovableTarget_C"))
  (Variables|Default|SetMovableTarget (Utilities|Array|Get(acopy) _outactors))
  ;[1 1 1] Set time actors
  (bind _outactors_2 (Actor|GetAllActorswithInterface "/Game/Blueprints/Interface/BPI_TimeRemaining.BPI_TimeRemaining_C"))
  (Variables|Default|SetTimeActor (Utilities|Array|Get(acopy) _outactors_2))
  ;[1 1 1] Load high score
  (bind _returnvalue (SaveGame|CreateSaveGameObject "/Game/Blueprints/Core/SaveScore.SaveScore_C"))
  (bind _assave_score (Utilities|Casting|CastToSaveScore _returnvalue))
  (bind _output_get (Variables|Default|SetSaveObject _assave_score))
  (bind _returnvalue_2 (SaveGame|LoadGamefromSlot (Variables|/Game/Blueprints/Core/SaveScore.SaveScore_C|GetUserName _output_get) (Variables|/Game/Blueprints/Core/SaveScore.SaveScore_C|GetUserIndex _output_get)))
  (bind _assave_score_2 (Utilities|Casting|CastToSaveScore _returnvalue_2))
  ;[1 1 1] Update High Score
  (bind _outactors_3 (Actor|GetAllActorswithInterface "/Game/Blueprints/Interface/BPI_HighScore.BPI_HighScore_C"))
  (bind _ashigh_score_actor (Utilities|Casting|CastToHighScoreActor (Utilities|Array|Get(acopy) _outactors_3)))
  (Default|UpdateHighScore _ashigh_score_actor (Variables|/Game/Blueprints/Core/SaveScore.SaveScore_C|GetMaxScore _assave_score_2)))

(event EventStartGame
  (bind _movabletarget (Variables|Default|GetMovableTarget))
  (bind _asvrcharacter_bp (Utilities|Casting|CastToVRCharacter_BP (Game|Player|GetPlayerPawn 0)))
  (Default|SetCanScore _asvrcharacter_bp true)
  (Class|BPIMovableTarget|StartMoving(Message) _movabletarget)
  (bind _output_get (Variables|Default|SetSeconds 60))
  (Class|BPITimeRemaining|UpdateTime(Message) (Variables|Default|GetTimeActor) _output_get :!label _label)
  ;[1 1 1] Timer
  (if (> (Variables|Default|GetSeconds) 0)
    (Utilities|FlowControl|Delay 1.0)
    (Variables|Default|SetSeconds (- (Variables|Default|GetSeconds) 1))
    (goto _label)
    (else
      (Class|BPIMovableTarget|StopMoving(Message) _movabletarget)
      (Default|SetCanScore _asvrcharacter_bp false)
      (if (> (Variables|/Game/Blueprints/VRCharacter_BP.VRCharacter_BP_C|GetScore _asvrcharacter_bp) (Variables|/Game/Blueprints/Core/SaveScore.SaveScore_C|GetMaxScore (stale EventBeginPlay _assave_score_2)))
        ;[1 1 1] Save high score
        (bind _returnvalue (SaveGame|CreateSaveGameObject "/Game/Blueprints/Core/SaveScore.SaveScore_C"))
        (bind _assave_score (Utilities|Casting|CastToSaveScore _returnvalue))
        (bind _output_get_2 (Variables|Default|SetSaveObject _assave_score))
        (Variables|/Game/Blueprints/Core/SaveScore.SaveScore_C|SetMaxScore _output_get_2 (Variables|/Game/Blueprints/VRCharacter_BP.VRCharacter_BP_C|GetScore _asvrcharacter_bp))
        (SaveGame|SaveGametoSlot (Variables|Default|GetSaveObject) (Variables|/Game/Blueprints/Core/SaveScore.SaveScore_C|GetUserName (Variables|Default|GetSaveObject)) (Variables|/Game/Blueprints/Core/SaveScore.SaveScore_C|GetUserIndex (Variables|Default|GetSaveObject)))))))

(fn ConstructionScript)